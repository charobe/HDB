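; Player character Blueprint that handles level entry and exit with a capsule transition effect.
; BeginPlay fades the screen out, shows a Stage01 widget on that map, and, unless the game instance's IntoStage is set, shrinks the capsule with Niagara dissolve before restoring input.
; GetSerum or debug-style map inputs lock input, grow the capsule via timelines, fade in and open Stage02 or BossRoom.
; Tick opens Retry_Clear after a delay once Clear is set.
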(event `self.ReceiveTick`
  (params (DeltaSeconds :type "Float (single-precision)"))
  (if (`self.Clear`)
    (`KismetSystemLibrary.Delay` 3.0)
    (`GameplayStatics.OpenLevelBySoftObjectPtr` "/Game/HDB/Map/Retry_Clear.Retry_Clear")))

(event `GetSerum`
  (`self.DisableInput` (`GameplayStatics.GetPlayerController` 0) :!label _label)
  (`SceneComponent.SetHiddenInGame` (`self.ChangeCapsule`) false false)
  (bind (_direction _growalpha) (`Timeline|CapsuleGrow`)
    (:`Update`
      (`SceneComponent.SetWorldScale3D` (`self.ChangeCapsule`) (`KismetMathLibrary.VLerp` (1.0 1.0 0.1) (1.0 1.0 1.0) _growalpha)))
    (:`Finished`
      (bind _returnvalue (`|CreateWidget` "/Game/HDB/UI/WBP_FadeScreen.WBP_FadeScreen_C"))
      (`UserWidget.AddToViewport` _returnvalue 0)
      (`/Game/HDB/UI/WBP_FadeScreen.FadeIn` _returnvalue)
      (`KismetSystemLibrary.Delay` 1.0)
      (`GameplayStatics.OpenLevelBySoftObjectPtr` "/Game/HDB/Map/NewMap/Stage02.Stage02")
      (`self.EnableInput` (`GameplayStatics.GetPlayerController` 0)))))

(event `InputAction|GoTo2Map`
  (params (Key :type "Key Structure"))
  (:`Pressed`
    (goto _label)))

(event `InputAction|GoToBossMap`
  (params (Key :type "Key Structure"))
  (:`Pressed`
    (`self.DisableInput` (`GameplayStatics.GetPlayerController` 0))
    (`SceneComponent.SetHiddenInGame` (`self.ChangeCapsule`) false false)
    (bind (_direction _growalpha) (`Timeline|Timeline`)
      (:`Update`
        (`SceneComponent.SetWorldScale3D` (`self.ChangeCapsule`) (`KismetMathLibrary.VLerp` (1.0 1.0 0.1) (1.0 1.0 1.0) _growalpha)))
      (:`Finished`
        (bind _returnvalue (`|CreateWidget` "/Game/HDB/UI/WBP_FadeScreen.WBP_FadeScreen_C"))
        (`UserWidget.AddToViewport` _returnvalue 0)
        (`/Game/HDB/UI/WBP_FadeScreen.FadeIn` _returnvalue)
        (`KismetSystemLibrary.Delay` 1.0)
        (`GameplayStatics.OpenLevelBySoftObjectPtr` "/Game/HDB/Map/NewMap/BossRoom.BossRoom")
        (`self.EnableInput` (`GameplayStatics.GetPlayerController` 0))))))

(event `self.ReceiveBeginPlay`
  (`self.DisableInput` (`GameplayStatics.GetPlayerController` 0))
  (`SceneComponent.SetHiddenInGame` (`self.ChangeCapsule`) false false)
  (bind _returnvalue (`|CreateWidget` "/Game/HDB/UI/WBP_FadeScreen.WBP_FadeScreen_C"))
  (`UserWidget.AddToViewport` _returnvalue 0)
  (`/Game/HDB/UI/WBP_FadeScreen.FadeOut` _returnvalue)
  (`KismetSystemLibrary.Delay` 1.0)
  (bind _returnvalue_2 (`GameplayStatics.GetCurrentLevelName` true))
  (if (`KismetStringLibrary.EqualEqual_StrStr` _returnvalue_2 "Stage01")
    (`KismetSystemLibrary.Delay` 8.0)
    (bind _returnvalue_3 (`|CreateWidget` "/Game/HDB/UI/WBP_Stage1.WBP_Stage1_C"))
    (`UserWidget.AddToViewport` _returnvalue_3 0))
  (bind _asbp_hdbgame_instance (cast `/Game/HDB/BluePrint/BP_HDBGameInstance` (`GameplayStatics.GetGameInstance`)))
  (if (not (`/Game/HDB/BluePrint/BP_HDBGameInstance.IntoStage` _asbp_hdbgame_instance))
    (set `/Game/HDB/BluePrint/BP_HDBGameInstance.IntoStage` false _asbp_hdbgame_instance)
    (bind (_direction _growalpha) (`Timeline|Timeline_0`)
      (:`Update`
        (`self.DissolveCapsuleEvent`)
        (`SceneComponent.SetWorldScale3D` (`self.ChangeCapsule`) (`KismetMathLibrary.VLerp` (1.0 1.0 1.0) (1.0 1.0 0.0) _growalpha)))
      (:`Finished`
        (`SceneComponent.SetHiddenInGame` (`self.ChangeCapsule`) true false)
        (`self.EnableInput` (`GameplayStatics.GetPlayerController` 0))))))

(event `DissolveCapsuleEvent`
  (`NiagaraFunctionLibrary.SpawnSystemAtLocation` "/Game/Asset/Effect/DissolveCapsule/NS_DissolveCapsule.NS_DissolveCapsule" (+ (`self.K2_GetActorLocation`) (0.0 0.0 -75.0))))

(fn `UserConstructionScript`)