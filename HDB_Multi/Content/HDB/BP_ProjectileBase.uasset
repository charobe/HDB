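; Base projectile Blueprint that handles audio and impact effects, with no movement, collision or damage logic in its graphs.
; On BeginPlay it plays a spawn sound at its location and spawns an attached flight sound that stops when the projectile is destroyed.
; A SpawnHitFX event, not called within these graphs, plays a sound and spawns a Niagara system at the given hit location, skipping any unset asset.
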(event `self.ReceiveBeginPlay`
  (`|ExecutionSequence`
    (:`then_0`
      (bind _projectile_spawn_sound (`self.Projectile Spawn Sound`)
        (:`then`
          (`GameplayStatics.PlaySoundAtLocation` _projectile_spawn_sound (`self.K2_GetActorLocation`) (struct) 1.0 1.0 0.0 null null null null))
        (:`else`)))
    (:`then_1`
      (bind _projectile_fly_sound (`self.Projectile Fly Sound`)
        (:`then`
          (`GameplayStatics.SpawnSoundAttached` _projectile_fly_sound null "None" (0.0 0.0 0.0) (struct) "KeepRelativeOffset" true 1.0 1.0 0.0 null null))
        (:`else`)))))

(event `self.BP_SpawnHitFX`
  (params (HitLocation :type "Vector Structure (by ref)"))
  (`|ExecutionSequence`
    (:`then_0`
      (bind _sound (`self.Sound`)
        (:`then`
          (`GameplayStatics.PlaySoundAtLocation` _sound HitLocation (struct) 1.0 1.0 0.0 null null null null))
        (:`else`)))
    (:`then_1`
      (bind _system_template (`self.System Template`)
        (:`then`
          (`NiagaraFunctionLibrary.SpawnSystemAtLocation` _system_template HitLocation))
        (:`else`)))))

(fn `UserConstructionScript`)