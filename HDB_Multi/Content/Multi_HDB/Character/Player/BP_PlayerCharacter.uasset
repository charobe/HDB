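; Multiplayer player character Blueprint that handles level-specific UI and map travel.
; BeginPlay shows start, result or clear-result widgets by level name, setting cursor and input mode to match.
; Request events cast the game mode, set a travelling flag against repeats, then ServerTravel on authority to stages, boss room, lobby or result maps.
; GoTo inputs trigger clear, Stage02 and boss travel; debug-style keys host Lab or join a hardcoded IP.
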(event `self.ReceiveBeginPlay`
  (bind _returnvalue (`GameplayStatics.GetPlayerController` 0))
  (bind _returnvalue_2 (`GameplayStatics.GetPlayerController` 0))
  (bind _returnvalue_3 (`GameplayStatics.GetPlayerController` 0))
  (bind _returnvalue_4 (`GameplayStatics.GetPlayerController` 0))
  (bind _returnvalue_5 (`GameplayStatics.GetCurrentLevelName` true))
  (if (`KismetStringLibrary.EqualEqual_StrStr` _returnvalue_5 "Lab")
    (bind _returnvalue_6 (`|CreateWidget` "/Game/Multi_HDB/Widget/GameModeWidget/WBP_Start.WBP_Start_C"))
    (`UserWidget.AddToViewport` _returnvalue_6 0)
    (set `PlayerController.bShowMouseCursor` true _returnvalue_2)
    (`WidgetBlueprintLibrary.SetInputMode_GameAndUIEx` _returnvalue_2 null)
    (else
      (bind _returnvalue_7 (`GameplayStatics.GetCurrentLevelName` true))
      (if (`KismetStringLibrary.EqualEqual_StrStr` _returnvalue_7 "Retry")
        (bind _returnvalue_8 (`|CreateWidget` "/Game/Multi_HDB/Widget/GameModeWidget/WBP_Result.WBP_Result_C"))
        (`UserWidget.AddToViewport` _returnvalue_8 0)
        (set `PlayerController.bShowMouseCursor` true _returnvalue_3)
        (`WidgetBlueprintLibrary.SetInputMode_UIOnlyEx` _returnvalue_3 null)
        (else
          (bind _returnvalue_9 (`GameplayStatics.GetCurrentLevelName` true))
          (if (`KismetStringLibrary.EqualEqual_StrStr` _returnvalue_9 "Retry_Clear")
            (bind _returnvalue_10 (`|CreateWidget` "/Game/Multi_HDB/Widget/GameModeWidget/WBP_ClearResult.WBP_ClearResult_C"))
            (`UserWidget.AddToViewport` _returnvalue_10 0)
            (set `PlayerController.bShowMouseCursor` true _returnvalue_4)
            (`WidgetBlueprintLibrary.SetInputMode_UIOnlyEx` _returnvalue_4 null)
            (else
              (set `PlayerController.bShowMouseCursor` false _returnvalue)
              (`WidgetBlueprintLibrary.SetInputMode_GameOnly` _returnvalue))))))))

(event `Request1`
  (bind _asbp_game_mode_base (cast `/Game/Multi_HDB/GameMode/BP_GameModeBase` (`GameplayStatics.GetGameMode`)))
  (if (not (`/Game/Multi_HDB/GameMode/BP_GameModeBase.bIsTravelling` _asbp_game_mode_base))
    (set `/Game/Multi_HDB/GameMode/BP_GameModeBase.bIsTravelling` true _asbp_game_mode_base)
    (`/Engine/EditorBlueprintResources/ActorMacros.Switch Has Authority`
      (:`Authority`
        (`KismetSystemLibrary.K2_SetTimerDelegate` :`Time` 0.2)
        (`KismetSystemLibrary.ExecuteConsoleCommand` "ServerTravel /Game/HDB/Map/NewMap/Stage01?listen" null)))))

(event `InputAction|GoTo1`
  (params (Key :type "Key Structure"))
  (:`Pressed`
    (`self.RequestClear`)))

(event `InputAction|GoTo2`
  (params (Key :type "Key Structure"))
  (:`Pressed`
    (`self.RequestServer`)))

(event `RequestServer`
  (bind _asbp_game_mode_base (cast `/Game/Multi_HDB/GameMode/BP_GameModeBase` (`GameplayStatics.GetGameMode`)))
  (if (not (`/Game/Multi_HDB/GameMode/BP_GameModeBase.bIsTravelling` _asbp_game_mode_base))
    (set `/Game/Multi_HDB/GameMode/BP_GameModeBase.bIsTravelling` true _asbp_game_mode_base)
    (`/Engine/EditorBlueprintResources/ActorMacros.Switch Has Authority`
      (:`Authority`
        (`KismetSystemLibrary.K2_SetTimerDelegate` :`Time` 0.2)
        (`KismetSystemLibrary.ExecuteConsoleCommand` "ServerTravel /Game/HDB/Map/NewMap/Stage02?listen" null)))))

(event `InputAction|GoTo3`
  (params (Key :type "Key Structure"))
  (:`Pressed`
    (`self.Request3`)))

(event `Request3`
  (bind _asbp_survival_game_mode (cast `/Game/Multi_HDB/GameMode/BP_SurvivalGameMode` (`GameplayStatics.GetGameMode`)))
  (if (not (`/Game/Multi_HDB/GameMode/BP_SurvivalGameMode.bIsTraveling2` _asbp_survival_game_mode))
    (set `/Game/Multi_HDB/GameMode/BP_SurvivalGameMode.bIsTraveling2` true _asbp_survival_game_mode)
    (`/Engine/EditorBlueprintResources/ActorMacros.Switch Has Authority`
      (:`Authority`
        (`KismetSystemLibrary.K2_SetTimerDelegate` :`Time` 0.2)
        (`KismetSystemLibrary.ExecuteConsoleCommand` "ServerTravel /Game/HDB/Map/NewMap/BossRoom?listen" null)))))

(event `Key|Two`
  (params (Key :type "Key Structure"))
  (:`Pressed`
    (`KismetSystemLibrary.ExecuteConsoleCommand` "open 192.168.67.92:7777" null)))

(event `Key|One`
  (params (Key :type "Key Structure"))
  (:`Pressed`
    (`GameplayStatics.OpenLevelBySoftObjectPtr` "/Game/HDB/Map/NewMap/Lab.Lab" true "listen")))

(event `RequestRetry`
  (bind _asbp_game_mode_base (cast `/Game/Multi_HDB/GameMode/BP_GameModeBase` (`GameplayStatics.GetGameMode`)))
  (if (not (`/Game/Multi_HDB/GameMode/BP_GameModeBase.bIsTravelling` _asbp_game_mode_base))
    (set `/Game/Multi_HDB/GameMode/BP_GameModeBase.bIsTravelling` true _asbp_game_mode_base)
    (`/Engine/EditorBlueprintResources/ActorMacros.Switch Has Authority`
      (:`Authority`
        (`KismetSystemLibrary.K2_SetTimerDelegate` :`Time` 0.2)
        (`KismetSystemLibrary.ExecuteConsoleCommand` "ServerTravel /Game/HDB/Map/Retry?listen" null)))))

(event `RequestClear`
  (bind _asbp_game_mode_base (cast `/Game/Multi_HDB/GameMode/BP_GameModeBase` (`GameplayStatics.GetGameMode`)))
  (if (not (`/Game/Multi_HDB/GameMode/BP_GameModeBase.bIsTravelling` _asbp_game_mode_base))
    (set `/Game/Multi_HDB/GameMode/BP_GameModeBase.bIsTravelling` true _asbp_game_mode_base)
    (`/Engine/EditorBlueprintResources/ActorMacros.Switch Has Authority`
      (:`Authority`
        (`KismetSystemLibrary.K2_SetTimerDelegate` :`Time` 0.2)
        (`KismetSystemLibrary.ExecuteConsoleCommand` "ServerTravel /Game/HDB/Map/Retry_Clear?listen" null)))))

(event `RequestLobby`
  (bind _asbp_game_mode_base (cast `/Game/Multi_HDB/GameMode/BP_GameModeBase` (`GameplayStatics.GetGameMode`)))
  (if (not (`/Game/Multi_HDB/GameMode/BP_GameModeBase.bIsTravelling` _asbp_game_mode_base))
    (set `/Game/Multi_HDB/GameMode/BP_GameModeBase.bIsTravelling` true _asbp_game_mode_base)
    (`/Engine/EditorBlueprintResources/ActorMacros.Switch Has Authority`
      (:`Authority`
        (`KismetSystemLibrary.K2_SetTimerDelegate` :`Time` 0.2)
        (`KismetSystemLibrary.ExecuteConsoleCommand` "ServerTravel /Game/HDB/Map/NewMap/Lab?listen" null)))))

(fn `UserConstructionScript`)