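; GA_Boss_Hitreact is the gameplay ability for the Golem boss's hit reaction, showing a decal on the side that was struck.
; When activated from an event, it takes the impact point from the event's first target-data hit result.
; It compares squared distances to the mesh's Decal_L and Decal_R sockets, passes the left-or-right result to BP_Golem's ShowDecal, then ends.
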(event `self.K2_ActivateAbility`)

(event `self.K2_ActivateAbilityFromEvent`
  (params (EventData :type "GameplayEventData Structure (by ref)"))
  (bind (_bblockinghit _binitialoverlap _time _distance _location _impactpoint) (`GameplayStatics.BreakHitResult` (`AbilitySystemBlueprintLibrary.GetHitResultFromTargetData` (`.TargetData` (break `GameplayEventData` EventData)))))
  (`|ExecutionSequence`
    (:`then_3`
      (bind _asbp_golem (cast `/Game/Multi_HDB/Character/Enemy/Golem/BP_Golem` (`self.GetAvatarActorFromActorInfo`)))
      (bind _mesh (`Character.Mesh` _asbp_golem))
      (`/Game/Multi_HDB/Character/Enemy/Golem/BP_Golem.ShowDecal` _asbp_golem (< (`KismetMathLibrary.Vector_DistanceSquared` _impactpoint (`SceneComponent.GetSocketLocation` _mesh "Decal_L")) (`KismetMathLibrary.Vector_DistanceSquared` _impactpoint (`SceneComponent.GetSocketLocation` _mesh "Decal_R"))) (0.0 0.0 0.0))
      (`self.K2_EndAbility`))))