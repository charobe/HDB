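; Golem enemy Blueprint that manages two sets of four decals, one for the left side and one for the right.
; ShowDecal takes a left/right flag, unhides that side's decal at the current index, then advances the index, wrapping after four.
; BeginPlay gathers the decals into per-side arrays, but ShowDecal references each component directly.
; Nothing in these graphs calls ShowDecal or re-hides the decals.
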(event `self.ReceiveBeginPlay`
  (`parent.ReceiveBeginPlay`)
  (set `self.LeftDecal` (`|MakeArray` (`self.DecalL1`) (`self.DecalL2`) (`self.DecalL3`) (`self.DecalL4`)))
  (set `self.RightDecal` (`|MakeArray` (`self.DecalR1`) (`self.DecalR2`) (`self.DecalR3`) (`self.DecalR4`))))

(fn `ShowDecal`
  (params (bLeft :type Boolean))
  (if bLeft
    (switch `int` (`self.LeftIndex`)
      (:`0`
        (`SceneComponent.SetHiddenInGame` (`self.DecalL1`) false false))
      (:`1`
        (`SceneComponent.SetHiddenInGame` (`self.DecalL2`) false false))
      (:`2`
        (`SceneComponent.SetHiddenInGame` (`self.DecalL3`) false false))
      (:`3`
        (`SceneComponent.SetHiddenInGame` (`self.DecalL4`) false false)))
    (set `self.LeftIndex` (mod (+ (`self.LeftIndex`) 1) 4))
    (else
      (switch `int` (`self.RightIndex`)
        (:`0`
          (`SceneComponent.SetHiddenInGame` (`self.DecalR1`) false false))
        (:`1`
          (`SceneComponent.SetHiddenInGame` (`self.DecalR2`) false false))
        (:`2`
          (`SceneComponent.SetHiddenInGame` (`self.DecalR3`) false false))
        (:`3`
          (`SceneComponent.SetHiddenInGame` (`self.DecalR4`) false false)))
      (set `self.RightIndex` (mod (+ (`self.RightIndex`) 1) 4)))))

(fn `UserConstructionScript`
  (`parent.UserConstructionScript`))