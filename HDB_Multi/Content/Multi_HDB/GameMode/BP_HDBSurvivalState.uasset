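; Survival-mode state Blueprint that shows on-screen wave announcements as the survival state changes.
; On BeginPlay it binds to OnSurvivalStateChanged and switches on the new state.
; Waiting for a new wave creates a countdown widget with a Korean "new wave approaching" message.
; Spawning a wave shows, after a short delay, a text widget with the current wave number.
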(event `self.ReceiveBeginPlay`
  (add `self.OnSurvivalStateChanged` (delegate `OnSurvivalStateChanged_Event`)))

(event `OnSurvivalStateChanged_Event` :!signature `self.OnSurvivalStateChanged`
  (params (NewState :type "EHDBSurvialGameModeState Enum" :default "WaitSpawnNewWave"))
  (switch `EHDBSurvialGameModeState` NewState
    (:`WaitSpawnNewWave`
      (`self.CreateWaveWidgetWithCountDown` "새로운 Wave가 다가오고 있습니다!" 5.0))
    (:`SpawningNewWave`
      (`KismetSystemLibrary.Delay` 2.0)
      (`self.CreateWaveWidgetWithoutCountDown` (`|FormatText` "Wave {CurrentWaveCount}" (`self.CurrentWaveCount`))))))

(fn `CreateWaveWidgetWithCountDown`
  (params (TextToDisplay :type Text) (InTotalCountDownTime :type "Float (double-precision)"))
  (bind _returnvalue (`|GenericCreateObject` "/Game/Multi_HDB/Widget/GameModeWidget/WBP_WaveTextWithCountDown.WBP_WaveTextWithCountDown_C"))
  (`UserWidget.AddToViewport` _returnvalue 0)
  (`TextBlock.SetText` (`/Game/Multi_HDB/Widget/GameModeWidget/WBP_WaveTextWithCountDown.WaveText` _returnvalue) (`local.TextToDisplay`))
  (`/Game/Multi_HDB/Widget/GameModeWidget/WBP_WaveTextWithCountDown.StartCountDown` _returnvalue (`local.InTotalCountDownTime`)))

(fn `CreateWaveWidgetWithoutCountDown`
  (params (Text :type Text))
  (bind _returnvalue (`|CreateWidget` "/Game/Multi_HDB/Widget/GameModeWidget/WBP_WaveTextWithoutCountDown.WBP_WaveTextWithoutCountDown_C"))
  (`UserWidget.AddToViewport` _returnvalue 0)
  (`TextBlock.SetText` (`/Game/Multi_HDB/Widget/GameModeWidget/WBP_WaveTextWithoutCountDown.WaveText` _returnvalue) (`local.Text`)))

(fn `UserConstructionScript`)