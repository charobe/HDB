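; BP_FieldObject is a scatter actor that fills a square field around its origin with randomly placed static mesh components.
; Its construction script loops up to Number, randomly picking one of three mesh component branches and offsetting it in X and Y within plus or minus Range.
; The random calls are unseeded, so the layout re-rolls whenever construction reruns, and the event graph has no active logic.
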(fn `UserConstructionScript`
  (bind _range (`self.Range`))
  (bind _returnvalue (* _range -1.0))
  (bind _returnvalue_2 (`KismetMathLibrary.MakeTransform` (`KismetMathLibrary.MakeVector` (`KismetMathLibrary.RandomFloatInRange` _returnvalue _range) (`KismetMathLibrary.RandomFloatInRange` _returnvalue _range))))
  (for _ (range (+ (`self.Number`) 1))
    (switch `int` (`KismetMathLibrary.RandomInteger` 3)
      (:`0`
        (`AddComponent|NODE_AddStaticMeshComponent-0` :`RelativeTransform` _returnvalue_2))
      (:`1`
        (`AddComponent|NODE_AddStaticMeshComponent-1` :`RelativeTransform` _returnvalue_2))
      (:`2`
        (`AddComponent|NODE_AddStaticMeshComponent-2` :`RelativeTransform` _returnvalue_2)))))