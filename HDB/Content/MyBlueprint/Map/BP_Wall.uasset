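; BP_Wall is a map-building actor that builds a straight wall from repeated static mesh pieces.
; Its construction script takes a direction from the X component of WallEnd, so the wall runs only along the local X axis.
; It adds a mesh component every 100 units from the actor's origin to cover that length.
; The event graph holds no active logic.
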(fn `UserConstructionScript`
  (bind _wallend_x (`KismetMathLibrary.BreakVector` (`self.WallEnd`)))
  (set `self.WallDirection` (`KismetMathLibrary.GetDirectionUnitVector` (0.0 0.0 0.0) (`KismetMathLibrary.MakeVector` _wallend_x)))
  (for _index (range (+ (`KismetMathLibrary.FTrunc` (/ (`KismetMathLibrary.VSizeXY` (`KismetMathLibrary.MakeVector` _wallend_x)) 100.0)) 1))
    (`AddComponent|NODE_AddStaticMeshComponent-0` :`RelativeTransform` (`KismetMathLibrary.Conv_VectorToTransform` (* _index 100 (`self.WallDirection`))))))