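; BP_Wall is a procedural wall Blueprint that lays out static mesh segments in a straight line from its local origin to WallEnd.
; The Construction Script derives direction and rotation from WallEnd, then adds a mesh component at fixed intervals, each rotated along that direction.
; The segment count comes from the horizontal length only, while placement follows the full 3D direction.
; The event graph has no active logic.
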(fn `UserConstructionScript`
  (bind _wallend (`self.WallEnd`))
  (bind _output_get (set `self.WallDirection` (`KismetMathLibrary.GetDirectionUnitVector` (0.0 0.0 0.0) _wallend)))
  (set `self.Rotate` (`KismetMathLibrary.Conv_VectorToRotator` _output_get))
  (for _index (range (+ (`KismetMathLibrary.FTrunc` (/ (`KismetMathLibrary.VSizeXY` _wallend) 50.0)) 1))
    (`AddComponent|NODE_AddStaticMeshComponent-0` :`RelativeTransform` (`KismetMathLibrary.MakeTransform` (* _index 50 (`self.WallDirection`)) (`self.Rotate`)))))