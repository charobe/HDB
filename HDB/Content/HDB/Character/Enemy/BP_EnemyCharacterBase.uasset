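; Base enemy character Blueprint that handles the death sequence when OnEnemyDied fires.
; It pauses mesh animation, disables capsule collision and plays a timeline rate-scaled by TotalDissolveTime.
; The timeline drives the DissolveAmount material parameter on the body, while setting the equipped weapon's to a constant zero.
; On finish, it destroys the weapon from EnemyCombatComponent, then the enemy itself.
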(event `/Game/HDB/Character/Enemy/BPI_EnemyDeath.OnEnemyDied`
  (bind _returnvalue (`PawnCombatComponent.GetCharacterCurrentEquippedWeapon` (`self.EnemyCombatComponent`)))
  (bind _returnvalue_2 (`PawnCombatComponent.GetCharacterCurrentEquippedWeapon` (`self.EnemyCombatComponent`)))
  (`|ExecutionSequence`
    (:`then_0`
      (set `SkeletalMeshComponent.bPauseAnims` true (`self.Mesh`))
      (`PrimitiveComponent.SetCollisionEnabled` (`self.CapsuleComponent`) "NoCollision"))
    (:`then_1`
      (`TimelineComponent.SetPlayRate` (`self.Dissolve TimeLine`) (/ 1.0 (`self.TotalDissolveTime`)))
      (bind (_direction _normalizedfloattrack) (`Timeline|Dissolve TimeLine` :!via `PlayFromStart`)
        (:`Update`
          (`MeshComponent.SetScalarParameterValueOnMaterials` (`self.Mesh`) "DissolveAmount" _normalizedfloattrack)
          (`/Engine/EditorBlueprintResources/StandardMacros.IsValid` _returnvalue_2
            (:`Is Valid`
              (`MeshComponent.SetScalarParameterValueOnMaterials` (`HDBWeaponBase.WeaponMesh` _returnvalue_2) "DissolveAmount" 0.0))))
        (:`Finished`
          (`/Engine/EditorBlueprintResources/StandardMacros.IsValid` _returnvalue
            (:`Is Valid`
              (`self.K2_DestroyActor` _returnvalue))
            (:`Is Not Valid`
              _))
          (`self.K2_DestroyActor`))))))

(fn `UserConstructionScript`)