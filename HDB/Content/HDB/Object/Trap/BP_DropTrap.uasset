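; BP_DropTrap is a trap that moves its TrapThronThron component by an offset when an HDB player character overlaps its Box.
; The overlap records the start location, sets the offset target and starts a fast VInterpTo move on Tick.
; On arrival it waits two seconds, eases back more slowly and re-arms at the start.
; The Active flag blocks retriggering during the cycle, and the file shows no damage logic.
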(event `self.ReceiveBeginPlay`)

(event `self.ReceiveTick`
  (params (DeltaSeconds :type "Float (single-precision)"))
  (bind _targetlocation (`self.TargetLocation`))
  (bind _returnvalue (`KismetMathLibrary.VInterpTo` (`SceneComponent.RelativeLocation` (`self.TrapThron_Thron`)) _targetlocation DeltaSeconds (`self.Speed`)))
  (if (`self.Move`)
    (`SceneComponent.K2_SetRelativeLocation` (`self.TrapThron_Thron`) _returnvalue false false)
    (if (< (`KismetMathLibrary.Vector_Distance` _returnvalue _targetlocation) 1.0)
      (if (== (`self.TargetLocation`) (`self.StartLocation`))
        (set `self.Move` false)
        (set `self.Active` false)
        (else
          (set `self.Move` false)
          (`KismetSystemLibrary.Delay` 2.0)
          (set `self.TargetLocation` (`self.StartLocation`))
          (set `self.Speed` 2.0)
          (set `self.Move` true))))))

(event `self.Box.OnComponentBeginOverlap`
  (params (OverlappedComponent :type "PrimitiveComponent Object Reference") (OtherActor :type "Actor Object Reference") (OtherComp :type "PrimitiveComponent Object Reference") (OtherBodyIndex :type Integer) (bFromSweep :type Boolean) (SweepResult :type "HitResult Structure (by ref)"))
  (cast `/Game/HDB/Character/Player/BP_HDBCharacterPlayer` OtherActor)
  (if (not (`self.Active`))
    (bind _output_get (set `self.StartLocation` (`SceneComponent.RelativeLocation` (`self.TrapThron_Thron`))))
    (set `self.TargetLocation` (+ _output_get (`self.TargetOffset`)))
    (set `self.Speed` 10.0)
    (set `self.Active` true)
    (set `self.Move` true)))

(fn `UserConstructionScript`)