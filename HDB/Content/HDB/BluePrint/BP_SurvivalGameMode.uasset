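; Survival game mode Blueprint that shows on-screen Korean announcements as the wave-based fight changes state.
; On BeginPlay it binds to the game mode state-change event and switches on the new state.
; Waiting, wave-completed and all-waves-done states create a countdown text widget, while spawning creates a new-wave banner.
; When the final wave spawns, it also overrides the spawn delay and shows a second, delayed banner warning of tougher resistance.
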(event `self.ReceiveBeginPlay`
  (add `self.OnSurvivalGameModeStateChanged` (delegate `OnSurvivalGameModeStateChanged_Event`)))

(event `OnSurvivalGameModeStateChanged_Event` :!signature `self.OnSurvivalGameModeStateChanged`
  (params (CurrentState :type "EHDBSurvivalGameModeState Enum" :default "WaitSpawnNewWave"))
  (switch `EHDBSurvivalGameModeState` CurrentState
    (:`WaitSpawnNewWave`
      (`self.CreateWaveWidget` (`|FormatText` "적들이 몰려옵니다...")))
    (:`SpawningNewWave`
      (`self.CreateNewWaveWidget` (`|FormatText` "몰려드는 적들을 처치하세요"))
      (if (== (`self.CurrentWaveCount`) (`self.TotalWave`))
        (set `self.SpawnDelayTime` 4.0)
        (`KismetSystemLibrary.Delay` 2.0)
        (`self.CreateNewWaveWidget` "적들의 저항이 거세집니다")))
    (:`WaveCompleted`
      (`self.CreateWaveWidget` (`|FormatText` "다음 전투에 대비하세요")))
    (:`AllWavesDone`
      (`self.CreateWaveWidget` (`|FormatText` "강력한 적이 다가오고 있습니다")))))

(fn `CreateNewWaveWidget`
  (params (Text :type Text))
  (bind _returnvalue (`|CreateWidget` "/Game/HDB/UI/GameModeWidget/WBP_NewWave.WBP_NewWave_C"))
  (`UserWidget.AddToViewport` _returnvalue 0)
  (`TextBlock.SetText` (`/Game/HDB/UI/GameModeWidget/WBP_NewWave.TextBlock_WaveText` _returnvalue) (`local.Text`)))

(fn `CreateWaveWidget`
  (params (TextToDisplay :type Text))
  (bind _returnvalue (`|CreateWidget` "/Game/HDB/UI/GameModeWidget/WBP_WaveTextWithCountDown.WBP_WaveTextWithCountDown_C"))
  (`UserWidget.AddToViewport` _returnvalue 0)
  (`TextBlock.SetText` (`/Game/HDB/UI/GameModeWidget/WBP_WaveTextWithCountDown.TextBlock_WaveText` _returnvalue) (`local.TextToDisplay`)))

(fn `UserConstructionScript`)