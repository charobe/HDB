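; BP_PlayerController handles the pause menu toggle through the Pausemenu input action.
; When the game is running, it creates a new Pause widget, adds it to the viewport, switches to UI-only input, shows the cursor and pauses.
; When already paused, it unpauses and restores game-only input, leaving the widget and cursor untouched.
; BeginPlay enables input using player controller 0.
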(event `self.ReceiveBeginPlay`
  (`self.EnableInput` (`GameplayStatics.GetPlayerController` 0)))

(event `InputAction|Pausemenu`
  (params (Key :type "Key Structure"))
  (bind _returnvalue (`GameplayStatics.GetPlayerController` 0))
  (:`Pressed`
    (if (`GameplayStatics.IsGamePaused`)
      (`GameplayStatics.SetGamePaused` false)
      (`WidgetBlueprintLibrary.SetInputMode_GameOnly` (`GameplayStatics.GetPlayerController` 0))
      (else
        (bind _returnvalue_2 (`|CreateWidget` "/Game/HDB/UI/Pause.Pause_C" _returnvalue))
        (`UserWidget.AddToViewport` _returnvalue_2 0)
        (`WidgetBlueprintLibrary.SetInputMode_UIOnlyEx` _returnvalue null)
        (set `PlayerController.bShowMouseCursor` true _returnvalue)
        (`GameplayStatics.SetGamePaused` true)))))

(fn `UserConstructionScript`)